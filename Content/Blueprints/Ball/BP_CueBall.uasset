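; Cue ball actor for a VR pool game that can be aimed, shot and respawned after being pocketed.
; Aim and Unaim swap its translucent material; Shoot applies force from the VR pawn's two hand release locations and records the shot in GlobalVars.
; Overlapping a pocket-tagged component teleports it to SpawnLocation, toggling physics around the move.
; The grab, drop and shoot event bindings are present but disconnected.
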(event `self.ReceiveBeginPlay`
  ;[1 1 1] Shoot Ball
  (bind _asvrpawn (cast `/Game/Blueprints/VRPawn` (`GameplayStatics.GetPlayerPawn` 0)))
  ;[1 1 1] Respawn the Ball
  (add `PrimitiveComponent.OnComponentBeginOverlap` (`self.Ball`) (delegate `OnComponentBeginOverlap_Event_0`)))

(event `Aim`
  ;[1 1 1] Select Ball
  (`PrimitiveComponent.SetMaterial` (`self.Ball`) 0 "/Game/Blueprints/Ball/WhiteBallTranslucent.WhiteBallTranslucent"))

(event `Unaim`
  ;[1 1 1] De-select Ball
  (`PrimitiveComponent.SetMaterial` (`self.Ball`) 0 "/Game/Blueprints/Ball/WhiteBall.WhiteBall"))

(event `Shoot`
  ;[1 1 1] Shoot Ball
  (`PrimitiveComponent.AddForce` (`self.Ball`) (* (- (`/Game/Blueprints/VRPawn.ReleaseLocationLeft` (stale `self.ReceiveBeginPlay` _asvrpawn)) (`/Game/Blueprints/VRPawn.ReleaseLocationRight` (stale `self.ReceiveBeginPlay` _asvrpawn))) 1000.0) "None" true)
  (bind _asglobal_vars (cast `/Game/Blueprints/GlobalVars` (`GameplayStatics.GetGameInstance`)))
  (set `/Game/Blueprints/GlobalVars.shooting` true _asglobal_vars)
  (set `/Game/Blueprints/GlobalVars.lastShotGameTime` (`KismetSystemLibrary.GetGameTimeInSeconds`) _asglobal_vars))

(event `OnComponentBeginOverlap_Event_0`
  (params (OverlappedComponent :type "PrimitiveComponent Object Reference") (OtherActor :type "Actor Object Reference") (OtherComp :type "PrimitiveComponent Object Reference") (OtherBodyIndex :type Integer) (bFromSweep :type Boolean) (SweepResult :type "HitResult Structure (by ref)"))
  (bind _ball (`self.Ball`))
  ;[1 1 1] Respawn the Ball
  (if (`ActorComponent.ComponentHasTag` OtherComp "tag_pocket")
    (`PrimitiveComponent.SetSimulatePhysics` _ball false)
    (`SceneComponent.K2_SetWorldLocation` _ball (`self.spawnLocation`) false true)
    (`PrimitiveComponent.SetSimulatePhysics` _ball true)))

(event `self.ReceiveTick`
  (params (DeltaSeconds :type "Float (single-precision)")))

(event `self.ReceiveActorBeginOverlap`
  (params (OtherActor :type "Actor Object Reference")))

(fn `UserConstructionScript`)