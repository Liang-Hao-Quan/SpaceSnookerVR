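; BP_TargetBall is a target ball with replicated movement that scores and disappears when potted.
; Overlapping a component tagged as a pocket destroys the ball, adds its Points to Player 1's score in the GlobalVars game instance, flags a scoring shot and plays a sound.
; A separate overlap collision plays impact sounds against the arena or other target balls, using a Priority comparison and short cooldown to limit duplicate ball-to-ball sounds.
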(event `Destory`
  (params (OverlappedComponent :type "PrimitiveComponent Object Reference") (OtherActor :type "Actor Object Reference") (OtherComp :type "PrimitiveComponent Object Reference") (OtherBodyIndex :type Integer) (bFromSweep :type Boolean) (SweepResult :type "HitResult Structure (by ref)"))
  ;[1 1 1] Target ball potted
  (if (`ActorComponent.ComponentHasTag` OtherComp "tag_pocket")
    (`self.K2_DestroyActor`)
    (bind _asglobal_vars (cast `/Game/Blueprints/GlobalVars` (`GameplayStatics.GetGameInstance`)))
    (set `/Game/Blueprints/GlobalVars.Player1Score` (+ (`/Game/Blueprints/GlobalVars.Player1Score` _asglobal_vars) (`self.points`)) _asglobal_vars)
    (set `/Game/Blueprints/GlobalVars.lastShotHasScore` true _asglobal_vars)
    (`GameplayStatics.PlaySound2D` "/Game/Audios/scoreSoundEffect.scoreSoundEffect" 1.0 1.0 0.0 null null)))

(event `self.ReceiveBeginPlay`
  (`|ExecutionSequence`
    (:`then_0`
      (`self.SetReplicateMovement` true)
      (add `PrimitiveComponent.OnComponentBeginOverlap` (`self.targetBall`) (delegate `Destory`))
      (set `self.lastSoundCollisionTime` 0.0))
    (:`then_1`
      (add `PrimitiveComponent.OnComponentBeginOverlap` (`self.overlapCollision`) (delegate `Overlap`)))))

(event `Overlap`
  (params (OverlappedComponent :type "PrimitiveComponent Object Reference") (OtherActor :type "Actor Object Reference") (OtherComp :type "PrimitiveComponent Object Reference") (OtherBodyIndex :type Integer) (bFromSweep :type Boolean) (SweepResult :type "HitResult Structure (by ref)"))
  ;[1 1 1] Collision sound
  (bind _asbp_target_ball (cast `/Game/Blueprints/Ball/BP_TargetBall` OtherActor)
    (:`then`
      (if (> (- (`KismetSystemLibrary.GetGameTimeInSeconds`) (`self.lastSoundCollisionTime`)) 0.1)
        (if (< (`/Game/Blueprints/Ball/BP_TargetBall.priority` _asbp_target_ball) (`self.priority`))
          (`GameplayStatics.PlaySoundAtLocation` "/Game/Audios/ballCollisionSound.ballCollisionSound" (`SceneComponent.K2_GetComponentLocation` (`self.targetBall`)) (struct) 3.0 1.0 0.0 null null null)
          (set `self.lastSoundCollisionTime` (`KismetSystemLibrary.GetGameTimeInSeconds`)))))
    (:`CastFailed`
      (cast `/Game/Blueprints/Arena` OtherActor)
      (`GameplayStatics.PlaySoundAtLocation` "/Game/Audios/ballCollisionSound.ballCollisionSound" (`SceneComponent.K2_GetComponentLocation` (`self.targetBall`)) (struct) 3.0 1.0 0.0 null null null))))

(fn `UserConstructionScript`)