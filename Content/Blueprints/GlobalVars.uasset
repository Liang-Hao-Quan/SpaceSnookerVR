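; GlobalVars holds session and turn logic for a multiplayer ball-and-pocket shooting game.
; Advanced Sessions events host a listen server on playRoom or join the first session found, printing on failure.
; UpdateStep clears Shooting, then either decrements Steps after a miss, ending at zero with -1, or handles a score.
; A score sets GameEnd either way, returning 0 if any ball remains valid, otherwise 1.
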(event `HostSessionEvent`
  ;[1 1 1] Create an new session
  (`CreateSessionCallbackProxyAdvanced.CreateAdvancedSession` :`PlayerController` (`GameplayStatics.GetPlayerController` 0) :`PublicConnections` 10 :`PrivateConnections` 10
    (:`OnSuccess`
      (`GameplayStatics.OpenLevel` "playRoom" true "?listen"))
    (:`OnFailure`
      (`KismetSystemLibrary.PrintString` "Create Advanced Session Fails" true true (struct :`G` 0.66 :`B` 1.0 :`A` 1.0) 10.0))))

(event `JoinSessionEvent`
  (bind _returnvalue (`GameplayStatics.GetPlayerController` 0))
  ;[1 1 1] Try to join an existed session
  (bind _results (`FindSessionsCallbackProxyAdvanced.FindSessionsAdvanced` _returnvalue 10 false "AllServers")
    (:`OnSuccess`
      (`JoinSessionCallbackProxy.JoinSession` _returnvalue (`|GetArrayItem` _results)))
    (:`OnFailure`
      (`KismetSystemLibrary.PrintString` "Find Advanced Session Fails" true true (struct :`G` 0.66 :`B` 1.0 :`A` 1.0) 10.0))))

(fn `UpdateStep`
  (params (Balls :type "Array of Actor Object Reference"))
  (returns (gameStatus :type Integer))
  (set `self.shooting` false)
  (if (`self.lastShotHasScore`)
    ;[1 1 1] Has hit pockets
    (set `self.lastShotHasScore` false)
    (for _array_element (`local.Balls`)
      (if (`KismetSystemLibrary.IsValid` _array_element)
        (set `self.gameEnd` true)
        (return 0)))
    (set `self.gameEnd` true)
    (return 1)
    (else
      ;[1 1 1] Not hit pockets
      (bind _output_get (set `self.steps` (- (`self.steps`) 1)))
      (if (<= _output_get 0)
        (set `self.gameEnd` true)
        (return -1)))))