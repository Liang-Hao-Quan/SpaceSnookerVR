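; BP_CueBall is a VR cue ball that can be grabbed, shot, and pocketed.
; Its GrabComponent events swap the Ball material to chrome while grabbed and back to white on drop.
; On shoot, it applies a mass-independent force along the vector from the VRPawn's right to left hand release location, scaled by their separation.
; Overlapping a component tagged as a pocket destroys the actor.
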(event `self.ReceiveBeginPlay`
  (add `/Game/VRTemplate/Blueprints/GrabComponent.OnGrabbed` (`self.GrabComponent`) (delegate `Aim`))
  (add `/Game/VRTemplate/Blueprints/GrabComponent.OnDropped` (`self.GrabComponent`) (delegate `Unaim`))
  (bind _asvrpawn (cast `/Game/VRTemplate/Blueprints/VRPawn` (`GameplayStatics.GetPlayerPawn` 0)))
  (add `/Game/VRTemplate/Blueprints/GrabComponent.OnShoot` (`self.GrabComponent`) (delegate `Shoot`))
  (add `PrimitiveComponent.OnComponentBeginOverlap` (`self.Ball`) (delegate `OnComponentBeginOverlap_Event_0`)))

(event `Aim`
  (`PrimitiveComponent.SetMaterial` (`self.Ball`) 0 "/Game/StarterContent/Materials/M_Metal_Chrome.M_Metal_Chrome"))

(event `Unaim`
  (`PrimitiveComponent.SetMaterial` (`self.Ball`) 0 "/Game/Ball/WhiteBall.WhiteBall"))

(event `Shoot`
  (`PrimitiveComponent.AddForce` (`self.Ball`) (* (- (`/Game/VRTemplate/Blueprints/VRPawn.ReleaseLocationLeft` (stale `self.ReceiveBeginPlay` _asvrpawn)) (`/Game/VRTemplate/Blueprints/VRPawn.ReleaseLocationRight` (stale `self.ReceiveBeginPlay` _asvrpawn))) 1000.0) "None" true))

(event `self.ReceiveTick`
  (params (DeltaSeconds :type "Float (single-precision)")))

(event `self.ReceiveActorBeginOverlap`
  (params (OtherActor :type "Actor Object Reference")))

(event `OnComponentBeginOverlap_Event_0`
  (params (OverlappedComponent :type "PrimitiveComponent Object Reference") (OtherActor :type "Actor Object Reference") (OtherComp :type "PrimitiveComponent Object Reference") (OtherBodyIndex :type Integer) (bFromSweep :type Boolean) (SweepResult :type "HitResult Structure (by ref)"))
  (if (`ActorComponent.ComponentHasTag` OtherComp "tag_pocket")
    (`self.K2_DestroyActor`)))

(fn `UserConstructionScript`)