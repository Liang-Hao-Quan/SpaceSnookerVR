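; BP_AsteroidBelt is an animated asteroid belt actor that spins continuously.
; Each Tick yaws the belt mesh by RotateSpeed scaled by delta time.
; It also tumbles the individual asteroid meshes in three groups, each with its own fixed local rotation step per frame, so their spin rate depends on frame rate.
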(event `self.ReceiveTick`
  (params (DeltaSeconds :type "Float (single-precision)"))
  (`SceneComponent.K2_AddLocalRotation` (`self.SM_AsteroidBelt`) (`KismetMathLibrary.MakeRotator` 0.0 0.0 (* DeltaSeconds (`self.RotateSpeed`))) false false)
  (`SceneComponent.K2_AddLocalRotation` (`self.StaticMesh13`) (struct :`Pitch` -0.2 :`Yaw` 0.2 :`Roll` 0.3) false false)
  (`SceneComponent.K2_AddLocalRotation` (`self.StaticMesh1`) (struct :`Pitch` -0.2 :`Yaw` 0.2 :`Roll` 0.3) false false)
  (`SceneComponent.K2_AddLocalRotation` (`self.StaticMesh2`) (struct :`Pitch` -0.2 :`Yaw` 0.2 :`Roll` 0.3) false false)
  (`SceneComponent.K2_AddLocalRotation` (`self.StaticMesh4`) (struct :`Pitch` -0.2 :`Yaw` 0.2 :`Roll` 0.3) false false)
  (`SceneComponent.K2_AddLocalRotation` (`self.StaticMesh5`) (struct :`Pitch` -0.2 :`Yaw` 0.2 :`Roll` 0.3) false false)
  (`SceneComponent.K2_AddLocalRotation` (`self.StaticMesh9`) (struct :`Pitch` -0.2 :`Yaw` 0.2 :`Roll` 0.3) false false)
  (`SceneComponent.K2_AddLocalRotation` (`self.StaticMesh12`) (struct :`Pitch` -0.2 :`Yaw` 0.2 :`Roll` 0.3) false false)
  (`SceneComponent.K2_AddLocalRotation` (`self.StaticMesh16`) (struct :`Pitch` -0.2 :`Yaw` 0.2 :`Roll` 0.3) false false)
  (`SceneComponent.K2_AddLocalRotation` (`self.StaticMesh17`) (struct :`Pitch` -0.2 :`Yaw` 0.2 :`Roll` 0.3) false false)
  (`SceneComponent.K2_AddLocalRotation` (`self.StaticMesh19`) (struct :`Pitch` -0.2 :`Yaw` 0.2 :`Roll` 0.3) false false)
  (`SceneComponent.K2_AddLocalRotation` (`self.StaticMesh23`) (struct :`Pitch` -0.2 :`Yaw` 0.2 :`Roll` 0.3) false false)
  (`SceneComponent.K2_AddLocalRotation` (`self.StaticMesh25`) (struct :`Pitch` -0.2 :`Yaw` 0.2 :`Roll` 0.3) false false)
  (`SceneComponent.K2_AddLocalRotation` (`self.SM_AsteroidA`) (struct :`Pitch` -0.2 :`Yaw` 0.2 :`Roll` 0.3) false false)
  (`SceneComponent.K2_AddLocalRotation` (`self.SM_AsteroidB`) (struct :`Pitch` -0.2 :`Yaw` 0.2 :`Roll` 0.3) false false)
  (`SceneComponent.K2_AddLocalRotation` (`self.StaticMesh3`) (struct :`Pitch` 0.2 :`Roll` 0.1) false false)
  (`SceneComponent.K2_AddLocalRotation` (`self.StaticMesh6`) (struct :`Pitch` 0.2 :`Roll` 0.1) false false)
  (`SceneComponent.K2_AddLocalRotation` (`self.StaticMesh8`) (struct :`Pitch` 0.2 :`Roll` 0.1) false false)
  (`SceneComponent.K2_AddLocalRotation` (`self.StaticMesh11`) (struct :`Pitch` 0.2 :`Roll` 0.1) false false)
  (`SceneComponent.K2_AddLocalRotation` (`self.StaticMesh15`) (struct :`Pitch` 0.2 :`Roll` 0.1) false false)
  (`SceneComponent.K2_AddLocalRotation` (`self.StaticMesh21`) (struct :`Pitch` 0.2 :`Roll` 0.1) false false)
  (`SceneComponent.K2_AddLocalRotation` (`self.StaticMesh22`) (struct :`Pitch` 0.2 :`Roll` 0.1) false false)
  (`SceneComponent.K2_AddLocalRotation` (`self.StaticMesh7`) (struct :`Pitch` 1.0 :`Yaw` 0.3 :`Roll` 0.1) false false)
  (`SceneComponent.K2_AddLocalRotation` (`self.StaticMesh`) (struct :`Pitch` 1.0 :`Yaw` 0.3 :`Roll` 0.1) false false)
  (`SceneComponent.K2_AddLocalRotation` (`self.StaticMesh10`) (struct :`Pitch` 1.0 :`Yaw` 0.3 :`Roll` 0.1) false false)
  (`SceneComponent.K2_AddLocalRotation` (`self.StaticMesh27`) (struct :`Pitch` 1.0 :`Yaw` 0.3 :`Roll` 0.1) false false)
  (`SceneComponent.K2_AddLocalRotation` (`self.StaticMesh14`) (struct :`Pitch` 1.0 :`Yaw` 0.3 :`Roll` 0.1) false false)
  (`SceneComponent.K2_AddLocalRotation` (`self.StaticMesh18`) (struct :`Pitch` 1.0 :`Yaw` 0.3 :`Roll` 0.1) false false)
  (`SceneComponent.K2_AddLocalRotation` (`self.StaticMesh20`) (struct :`Pitch` 1.0 :`Yaw` 0.3 :`Roll` 0.1) false false)
  (`SceneComponent.K2_AddLocalRotation` (`self.StaticMesh24`) (struct :`Pitch` 1.0 :`Yaw` 0.3 :`Roll` 0.1) false false)
  (`SceneComponent.K2_AddLocalRotation` (`self.StaticMesh26`) (struct :`Pitch` 1.0 :`Yaw` 0.3 :`Roll` 0.1) false false))

(fn `UserConstructionScript`)